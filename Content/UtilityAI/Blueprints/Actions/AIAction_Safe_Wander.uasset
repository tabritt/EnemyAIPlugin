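; Utility AI action for BP_NPCSimple that either moves the NPC to the player or holds it in place.
; Evaluate subtracts MaxDistance over player distance from the parent score, clamped to 0–1, so utility rises as the player gets farther away.
; Execute approaches the player on a high score, otherwise targets the NPC's own location unless the GoToPlayer flag marks an approach underway.
; Debug prints report the score and completed moves.
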(event `self.Execute`
  (params (ControlledActor :type "Actor Object Reference"))
  (bind _returnvalue (`self.Evaluate` ControlledActor))
  (bind _asbp_npcsimple (cast `/Game/UtilityAI/Blueprints/BP_NPCSimple` ControlledActor))
  (if (>= _returnvalue 0.8)
    (`|AIMoveTo` ControlledActor _asbp_npcsimple (`Actor.K2_GetActorLocation` (`/Game/UtilityAI/Blueprints/BP_NPCSimple.PlayerCharacter` _asbp_npcsimple)) null 30.0
      (:`then`
        (set `self.GoToPlayer` true))
      (:`OnSuccess`
        (`KismetSystemLibrary.PrintString` null)
        (set `self.GoToPlayer` false)))
    (elif (not (`self.GoToPlayer`))
      (`|AIMoveTo` ControlledActor _asbp_npcsimple (`Actor.K2_GetActorLocation` _asbp_npcsimple) null 30.0
        (:`OnSuccess`
          (`KismetSystemLibrary.PrintString` null "Don't move"))))))

(fn `Evaluate`
  (params (ControlledActor :type "Actor Object Reference"))
  (returns (ReturnValue :type "Float (single-precision)"))
  (bind _returnvalue (`parent.Evaluate` ControlledActor))
  (bind _asbp_npcsimple (cast `/Game/UtilityAI/Blueprints/BP_NPCSimple` ControlledActor))
  (bind _returnvalue_2 (`KismetMathLibrary.FClamp` (- _returnvalue (/ (`self.MaxDistance`) (`KismetMathLibrary.VSize` (- (`Actor.K2_GetActorLocation` _asbp_npcsimple) (`Actor.K2_GetActorLocation` (`/Game/UtilityAI/Blueprints/BP_NPCSimple.PlayerCharacter` _asbp_npcsimple))))))))
  (`KismetSystemLibrary.PrintString` null (`KismetStringLibrary.Conv_DoubleToString` _returnvalue_2))
  (return _returnvalue_2))